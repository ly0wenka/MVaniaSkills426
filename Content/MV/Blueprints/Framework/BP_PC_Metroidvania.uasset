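; Metroidvania player controller that runs the hold-to-open black and white magic radial or selection menus and dismisses the learned-skill popup.
; Menu widgets are created at BeginPlay; holding input swaps one for the HUD and pauses, while release restores play.
; White magic requires the character's WMagicReady, with a gate so release only closes an opened menu.
; Only black magic plays slotted feedback; the white version is disconnected.
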(event `InputAction|BlackMagicMenu` :paused true
  (params (Key :type "Key Structure"))
  (bind _returnvalue (`GameplayStatics.GetPlayerController` 0))
  (bind _wbp_bmagic_menu (`self.WBP_BMagic_Menu`))
  (bind _wbp_bmagic_menu_2 (`self.WBP_BMagic_Menu`))
  ;[1 1 1] sHOW / hIDE BMM
  (:`Pressed`
    (bind _asmv_hud (cast `/Game/mv_hud` (`self.GetHUD`)))
    (bind _wbp_mv_hud (`/Game/mv_hud.WBP_MV_HUD` _asmv_hud))
    (`Widget.RemoveFromParent` _wbp_mv_hud)
    (`UserWidget.AddToViewport` _wbp_bmagic_menu 0)
    (`UserWidget.PlayAnimation` _wbp_bmagic_menu_2 (`/Game/WBP_BMagicMenu.BMagicMenuIntro` _wbp_bmagic_menu_2) 0.0 1 "Forward" 1.0 false)
    (`GameplayStatics.PlaySound2D` (`self.SFX_Menu_ON`) 1.0 1.0 0.0 null null)
    (`GameplayStatics.SetGamePaused` true)
    (`WidgetBlueprintLibrary.SetInputMode_GameAndUIEx` _returnvalue (`self.WBP_BMagic_Menu`)))
  (:`Released`
    (`UserWidget.AddToViewport` _wbp_mv_hud 0)
    (`Widget.RemoveFromParent` _wbp_bmagic_menu)
    (`GameplayStatics.PlaySound2D` (`self.SFX_Menu_OFF`) 1.0 1.0 0.0 null null)
    (`GameplayStatics.SetGamePaused` false)
    (`WidgetBlueprintLibrary.SetInputMode_GameOnly` _returnvalue)
    ;[1 1 1] ShowSturBurstUponSelection
    (if (`/Game/WBP_BMagicMenu.bSelectionMade` (`self.WBP_BMagic_Menu`))
      (`GameplayStatics.PlaySound2D` (`self.SFX_MagicSlotted`) 1.0 1.0 0.0 null null)
      (bind _asmv_hud_2 (cast `/Game/mv_hud` (`self.GetHUD`)))
      (bind _wbp_mv_hud_2 (`/Game/mv_hud.WBP_MV_HUD` _asmv_hud_2))
      (`UserWidget.PlayAnimation` _wbp_mv_hud_2 (`/Game/HUD.BMagicSlotted` _wbp_mv_hud_2) 0.0 1 "Forward" 1.0 false))))

(event `InputAction|WhiteMagicMenu` :paused true
  (params (Key :type "Key Structure"))
  (bind _returnvalue (`GameplayStatics.GetPlayerController` 0))
  (bind _wbp_wmagic_menu (`self.WBP_WMagic_Menu`))
  (bind _wbp_wmagic_menu_2 (`self.WBP_WMagic_Menu`))
  ;[1 1 1] sHOW / hIDE WMM
  (:`Pressed`
    (bind _asside_scroller_character (cast `/Game/SideScrollerBP/Blueprints/SideScrollerCharacter` (`GameplayStatics.GetPlayerCharacter` 0)))
    (if (`MVCharacter.bWMagicReady` _asside_scroller_character)
      (`|ExecutionSequence`
        (:`then_0`
          (bind _asmv_hud (cast `/Game/mv_hud` (`self.GetHUD`)))
          (bind _wbp_mv_hud (`/Game/mv_hud.WBP_MV_HUD` _asmv_hud))
          (`Widget.RemoveFromParent` _wbp_mv_hud)
          (`UserWidget.AddToViewport` _wbp_wmagic_menu 0)
          (`UserWidget.PlayAnimation` _wbp_wmagic_menu_2 (`/Game/WBP_WMagicMenu.WMagicMenuIntro` _wbp_wmagic_menu_2) 0.0 1 "Forward" 1.0 false)
          (`GameplayStatics.PlaySound2D` (`self.SFX_Menu_ON`) 1.0 1.0 0.0 null null)
          (`GameplayStatics.SetGamePaused` true)
          (`WidgetBlueprintLibrary.SetInputMode_GameAndUIEx` _returnvalue (`self.WBP_WMagic_Menu`)))
        (:`then_1`
          (goto _label :!via `Open`)))
      (else
        (`GameplayStatics.PlaySound2D` (`self.SFX_ActionDisallowed`) 0.3 1.0 0.0 null null))))
  (:`Released`
    (`/Engine/EditorBlueprintResources/StandardMacros.Gate` true :!label _label
      (:`Exit`
        (`|ExecutionSequence`
          (:`then_0`
            (`UserWidget.AddToViewport` _wbp_mv_hud 0)
            (`Widget.RemoveFromParent` _wbp_wmagic_menu)
            (`GameplayStatics.PlaySound2D` (`self.SFX_Menu_OFF`) 1.0 1.0 0.0 null null)
            (`GameplayStatics.SetGamePaused` false)
            (`WidgetBlueprintLibrary.SetInputMode_GameOnly` _returnvalue))
          (:`then_1`
            (goto _label :!via `Close`)))))))

(event `self.ReceiveBeginPlay`
  (`|ExecutionSequence`
    (:`then_0`
      ;[1 1 1] BMM Reference
      (bind _returnvalue (`|CreateWidget` "/Game/WBP_BMagicMenu.WBP_BMagicMenu_C"))
      (set `self.WBP_BMagic_Menu` _returnvalue))
    (:`then_1`
      ;[1 1 1] WMM Reference
      (bind _returnvalue_2 (`|CreateWidget` "/Game/WBP_WMagicMenu.WBP_WMagicMenu_C"))
      (set `self.WBP_WMagic_Menu` _returnvalue_2))))

(event `self.ShowAcquiredSkill`
  (`GameplayStatics.SetGamePaused` true)
  (`UserWidget.AddToViewport` (`self.WBP_LearnedSkill`) 0))

(event `InputAction|ExitSkillAcquire` :consume false :paused true
  (params (Key :type "Key Structure"))
  (bind _returnvalue (`GameplayStatics.GetPlayerController` 0))
  (:`Pressed`
    (if (`GameplayStatics.IsGamePaused`)
      (`/Engine/EditorBlueprintResources/StandardMacros.IsValid` (`self.WBP_LearnedSkill`)
        (:`Is Valid`
          (`Widget.RemoveFromParent` (`self.WBP_LearnedSkill`))
          (`GameplayStatics.SetGamePaused` false)
          (`WidgetBlueprintLibrary.SetInputMode_GameOnly` _returnvalue)
          (set `PlayerController.bShowMouseCursor` true _returnvalue))))))

(fn `UserConstructionScript`)