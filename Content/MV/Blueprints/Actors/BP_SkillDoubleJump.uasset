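; Double jump skill pickup actor for the side-scroller, with a mesh, VFX, light and interact collider.
; Overlapping the collider sets CanInteract on the SideScrollerCharacter; the interaction event is empty and no skill is granted here.
; PlayerAcquiredSkillFX removes the notify widget, plays an explosion emitter and acquire sound, then destroys those components, leaving the actor itself in place.
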(event `self.InteractColliderBox.OnComponentBeginOverlap`
  (params (OverlappedComponent :type "PrimitiveComponent Object Reference") (OtherActor :type "Actor Object Reference") (OtherComp :type "PrimitiveComponent Object Reference") (OtherBodyIndex :type Integer) (bFromSweep :type Boolean) (SweepResult :type "HitResult Structure (by ref)"))
  (bind _asside_scroller_character (cast `/Game/SideScrollerBP/Blueprints/SideScrollerCharacter` OtherActor))
  (set `MVCharacter.bCanInteract` true _asside_scroller_character)
  (if true
    _))

(event `self.PlayerAcquiredSkillFX`
  (`Widget.RemoveFromParent` (`self.Notify`))
  (`GameplayStatics.SpawnEmitterAtLocation` "/Game/InfinityBladeEffects/Effects/FX_Treasure/Resources/P_OrePile_Explosion_Success.P_OrePile_Explosion_Success" (`SceneComponent.K2_GetComponentLocation` (`self.Skill_Mesh`)) (struct) (2.0 2.0 2.0))
  (`GameplayStatics.PlaySound2D` (`self.SFX_SkillAcquire`) 3.0 1.0 0.0 null null)
  (`ActorComponent.K2_DestroyComponent` (`self.Skill_Mesh`))
  (`ActorComponent.K2_DestroyComponent` (`self.Skill_VFX`))
  (`ActorComponent.K2_DestroyComponent` (`self.Skill_Light`))
  (`ActorComponent.K2_DestroyComponent` (`self.InteractColliderBox`)))

(event `self.ObjectInteractedWith`)

(fn `UserConstructionScript`)