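; World pickup that grants the side-scroller player the Mist magic skill on interaction.
; Overlapping its collider enables interaction and, if the player neither has nor is using Mist, shows an animated prompt with sound.
; Interacting sets the character's skill state, plays burst effects and destroys the pickup's components.
; After a short delay, it passes a skill-acquired widget to the Metroidvania player controller for display.
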(event `self.InteractColliderBox.OnComponentBeginOverlap`
  (params (OverlappedComponent :type "PrimitiveComponent Object Reference") (OtherActor :type "Actor Object Reference") (OtherComp :type "PrimitiveComponent Object Reference") (OtherBodyIndex :type Integer) (bFromSweep :type Boolean) (SweepResult :type "HitResult Structure (by ref)"))
  (bind (_as_side_scroller_character _bhaswmagicmist) (`self.HasWMagicMist`))
  (bind _notify (`self.Notify`))
  ;[1 1 1] Show Interact Message
  (bind _asside_scroller_character (cast `/Game/SideScrollerBP/Blueprints/SideScrollerCharacter` OtherActor))
  (set `MVCharacter.bCanInteract` true _asside_scroller_character)
  (if _bhaswmagicmist
    _
    (elif (not (`MVCharacter.bIsUsingMist` _as_side_scroller_character))
      (set `/Game/Notify.ReceivedMessage` (`self.InteractMessage`) _notify)
      (`UserWidget.AddToViewport` _notify 0)
      (`UserWidget.PlayAnimation` _notify (`/Game/Notify.Intro` _notify) 0.0 1 "Forward" 1.0 false)
      (`GameplayStatics.PlaySound2D` (`self.SFXCanInteract`) 5.0 1.0 0.0 null null))))

(event `self.InteractColliderBox.OnComponentEndOverlap`
  (params (OverlappedComponent :type "PrimitiveComponent Object Reference") (OtherActor :type "Actor Object Reference") (OtherComp :type "PrimitiveComponent Object Reference") (OtherBodyIndex :type Integer))
  (bind _notify (`self.Notify`))
  (bind _intro (`/Game/Notify.Intro` _notify))
  ;[1 1 1] Hide Interact Message
  (cast `/Game/SideScrollerBP/Blueprints/SideScrollerCharacter` OtherActor)
  (`UserWidget.PlayAnimation` _notify _intro 0.0 1 "Reverse" 1.0 false)
  (`KismetSystemLibrary.Delay` (`WidgetAnimation.GetEndTime` _intro))
  (`Widget.RemoveFromParent` (`self.Notify`))
  (set `MVCharacter.bCanInteract` false (`self.As Side Scroller Character`)))

(event `self.ObjectInteractedWith`
  (bind (_as_side_scroller_character _bhaswmagicmist) (`self.HasWMagicMist`))
  ;[1 1 1] Player Acquires Mist
  (if _bhaswmagicmist
    (`KismetSystemLibrary.PrintString` "Player already has Mist.")
    (else
      (set `MVCharacter.bHasWMagicMist` true _as_side_scroller_character)
      (set `MVCharacter.SkillAcquired` "Mist" _as_side_scroller_character)
      (`self.PlayerAcquiredSkillFX`)
      (`KismetSystemLibrary.Delay` 0.75)
      (bind _returnvalue (`|CreateWidget` "/Game/SkillAcquired.SkillAcquired_C"))
      (bind _asbp_pc_metroidvania (cast `/Game/MV/Blueprints/Framework/BP_PC_Metroidvania` (`GameplayStatics.GetPlayerController` 0)))
      (set `MV_PC_Metroidvania.WBP_LearnedSkill` _returnvalue _asbp_pc_metroidvania)
      (`/Game/MV/Blueprints/Framework/BP_PC_Metroidvania.ShowAcquiredSkill` _asbp_pc_metroidvania))))

(fn `HasWMagicMist`
  (returns (`As Side Scroller Character` :type "/Game/SideScrollerBP/Blueprints/SideScrollerCharacter Object Reference") (bHasWMagicMist :type Boolean))
  (bind _as_side_scroller_character (`self.As Side Scroller Character`))
  (return _as_side_scroller_character (`MVCharacter.bHasWMagicMist` _as_side_scroller_character)))

(fn `PlayerAcquiredSkillFX`
  (`Widget.RemoveFromParent` (`self.Notify`))
  (`GameplayStatics.SpawnEmitterAtLocation` "/Game/InfinityBladeEffects/Effects/FX_Treasure/Resources/P_OrePile_Explosion_Success.P_OrePile_Explosion_Success" (`SceneComponent.K2_GetComponentLocation` (`self.Skill_Mesh`)) (struct) (2.0 2.0 2.0))
  (`GameplayStatics.PlaySound2D` (`self.SFX_SkillAcquire`) 3.0 1.0 0.0 null null)
  (`ActorComponent.K2_DestroyComponent` (`self.Skill_Mesh`))
  (`ActorComponent.K2_DestroyComponent` (`self.Skill_VFX`))
  (`ActorComponent.K2_DestroyComponent` (`self.Skill_Light`))
  (`ActorComponent.K2_DestroyComponent` (`self.InteractColliderBox`)))

(fn `UserConstructionScript`
  (`parent.UserConstructionScript`))