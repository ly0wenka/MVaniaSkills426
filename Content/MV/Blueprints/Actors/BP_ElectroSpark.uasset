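; BP_ElectroSpark is the actor for the ElectroSpark spell, damaging actors that overlap its collision.
; The overlap handler reads damage from the player MVCharacter's MagicMap and applies it to the overlapping actor.
; A DoOnce reset after a short delay limits damage to one hit per cooldown, shared across all targets.
; The Hit event is empty; Fireball-based impact effects, damage and destroy logic remain disconnected.
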(event `self.ReceiveHit`
  (params (MyComp :type "PrimitiveComponent Object Reference") (Other :type "Actor Object Reference") (OtherComp :type "PrimitiveComponent Object Reference") (bSelfMoved :type Boolean) (HitLocation :type "Vector Structure") (HitNormal :type "Vector Structure") (NormalImpulse :type "Vector Structure") (Hit :type "HitResult Structure (by ref)")))

(event `self.Collision.OnComponentBeginOverlap`
  (params (OverlappedComponent :type "PrimitiveComponent Object Reference") (OtherActor :type "Actor Object Reference") (OtherComp :type "PrimitiveComponent Object Reference") (OtherBodyIndex :type Integer) (bFromSweep :type Boolean) (SweepResult :type "HitResult Structure (by ref)"))
  (bind _asmvcharacter (cast `MVCharacter` (`GameplayStatics.GetPlayerCharacter` 0)))
  (`/Engine/EditorBlueprintResources/StandardMacros.DoOnce` false :!label _label
    (:`Completed`
      (`GameplayStatics.ApplyDamage` OtherActor (`.Damage` (break `STR_MagicAttributes` (`BlueprintMapLibrary.Map_Find` (`MVCharacter.MagicMap` _asmvcharacter) "ElectroSpark"))))
      (`KismetSystemLibrary.Delay` 2.1)
      (goto _label :!via `Reset`))))

(fn `UserConstructionScript`)